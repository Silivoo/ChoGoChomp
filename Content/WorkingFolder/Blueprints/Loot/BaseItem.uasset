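; BaseItem is a loot item actor that shows its name as text colored by rarity.
; On BeginPlay it looks up its ItemName row in DT_ArmorDataTable and, if found, writes the row's Name to a TextRender component.
; A Select on the row's Rarity picks the text color for each tier from Common to Exotic.
; The graphs contain no pickup or overlap logic.
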(event `self.ReceiveBeginPlay`
  (bind _textrender (`self.TextRender`))
  (bind _returnvalue (`|GetDataTableRow` "/Game/WorkingFolder/Blueprints/Loot/DT_ArmorDataTable.DT_ArmorDataTable" (`self.ItemName`))
    (:`then`
      (bind (_name _rarity) (break `/Game/WorkingFolder/Blueprints/Loot/DS_ArmorDataStruct` _returnvalue))
      (`TextRenderComponent.K2_SetText` _textrender (`KismetTextLibrary.Conv_NameToText` _name))
      (`TextRenderComponent.SetTextRenderColor` _textrender (select `/Game/WorkingFolder/Blueprints/Loot/ENUM_RarityEnum` _rarity :`NewEnumerator0` (make `Color` 0 0 0 100) :`NewEnumerator1` (make `Color` 49 212 49 100) :`NewEnumerator2` (make `Color` 255 213 0 100) :`NewEnumerator3` (make `Color` 212 49 190 100) :`NewEnumerator4` (make `Color` 31 209 215 100))))))

(fn `UserConstructionScript`)