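; BaseChest is a loot chest actor that spawns four random BaseItem pickups at offsets around itself, triggered from BeginPlay through SR_Open.
; Each drop rolls a rarity and an item type (gold, weapon or armor) using weighted Select tables over random integers.
; ChooseItem handles only armor: it rolls an armor type, filters DT_ArmorDataTable by type and rarity, then picks a random matching name for the spawned item.
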(event `self.ReceiveBeginPlay`
  (`self.SR_Open`))

(event `SR_Open`
  (for _index (range 4)
    (bind _rarityoutput (`self.ChooseRarity`))
    (bind _loottypeoutput (`self.ChooseItemType`))
    (bind _itemname (`self.ChooseItem` _loottypeoutput _rarityoutput))
    (`|SpawnActorFromClass` "/Game/WorkingFolder/Blueprints/Loot/BaseItem.BaseItem_C" (`KismetMathLibrary.MakeTransform` (+ (`|GetArrayItem` (`self.SpwanLocation`) _index) (`self.K2_GetActorLocation`))) "AlwaysSpawn" "OverrideRootScale" null _itemname null)))

(fn `ChooseArmorType`
  (returns (ArmorTypeOutput :type "/Game/WorkingFolder/Blueprints/Loot/ENUM_TypeOfArmorEnum Enum"))
  (return (select `int` (`KismetMathLibrary.RandomIntegerInRange` 0 6) :`0` "NewEnumerator0" :`1` "NewEnumerator1" :`2` "NewEnumerator2" :`3` "NewEnumerator6" :`4` "NewEnumerator3" :`5` "NewEnumerator4" :`6` "NewEnumerator5" :!type "/Game/WorkingFolder/Blueprints/Loot/ENUM_TypeOfArmorEnum Enum")))

(fn `ChooseItem`
  (params (ItemType :type "/Game/WorkingFolder/Blueprints/Loot/ENUM_LootTypeEnum Enum" :default "NewEnumerator0") (Rarity :type "/Game/WorkingFolder/Blueprints/Loot/ENUM_RarityEnum Enum" :default "NewEnumerator0"))
  (returns (ItemName :type Name))
  (locals (CompatibleItems :type "Array of Name"))
  (bind _compatibleitems (`local.CompatibleItems`))
  (switch `/Game/WorkingFolder/Blueprints/Loot/ENUM_LootTypeEnum` ItemType
    (:`NewEnumerator2`
      ;[1 0.7423 0.1661] ArmorLootSortDrop
      (bind _armortypeoutput (`self.ChooseArmorType`))
      (bind _outrownames (`DataTableFunctionLibrary.GetDataTableRowNames` null))
      (for _array_element _outrownames
        (bind _returnvalue (`|GetDataTableRow` "/Game/WorkingFolder/Blueprints/Loot/DT_ArmorDataTable.DT_ArmorDataTable" _array_element)
          (:`then`
            (bind (_name _rarity _armortype) (break `/Game/WorkingFolder/Blueprints/Loot/DS_ArmorDataStruct` _returnvalue))
            (if (and (== _rarity Rarity) (== _armortype _armortypeoutput))
              (`KismetArrayLibrary.Array_Add` (`local.CompatibleItems`) _name)))))
      (return (`|GetArrayItem` _compatibleitems (`KismetMathLibrary.RandomIntegerInRange` 0 (`KismetArrayLibrary.Array_LastIndex` _compatibleitems)))))))

(fn `ChooseItemType`
  (returns (LootTypeOutput :type "/Game/WorkingFolder/Blueprints/Loot/ENUM_LootTypeEnum Enum"))
  (return (select `int` (`KismetMathLibrary.RandomIntegerInRange` 0 9) :`0` "NewEnumerator0" :`1` "NewEnumerator0" :`2` "NewEnumerator0" :`3` "NewEnumerator0" :`4` "NewEnumerator1" :`5` "NewEnumerator1" :`6` "NewEnumerator1" :`7` "NewEnumerator2" :`8` "NewEnumerator2" :`9` "NewEnumerator2" :!type "/Game/WorkingFolder/Blueprints/Loot/ENUM_LootTypeEnum Enum")))

(fn `ChooseRarity`
  (returns (RarityOutput :type "/Game/WorkingFolder/Blueprints/Loot/ENUM_RarityEnum Enum"))
  (return (select `int` (`KismetMathLibrary.RandomIntegerInRange` 0 20) :`0` "NewEnumerator0" :`1` "NewEnumerator0" :`2` "NewEnumerator0" :`3` "NewEnumerator0" :`4` "NewEnumerator0" :`5` "NewEnumerator0" :`6` "NewEnumerator0" :`7` "NewEnumerator0" :`8` "NewEnumerator0" :`9` "NewEnumerator1" :`10` "NewEnumerator1" :`11` "NewEnumerator1" :`12` "NewEnumerator1" :`13` "NewEnumerator1" :`14` "NewEnumerator2" :`15` "NewEnumerator2" :`16` "NewEnumerator2" :`17` "NewEnumerator2" :`18` "NewEnumerator3" :`19` "NewEnumerator3" :`20` "NewEnumerator4" :!type "/Game/WorkingFolder/Blueprints/Loot/ENUM_RarityEnum Enum")))

(fn `UserConstructionScript`)